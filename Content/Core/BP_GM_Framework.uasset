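; Framework game mode that tracks connected player controllers and provides respawning of player characters.
; PostLogin, controller swaps and logout keep the AllPCs list of BP_PC_Framework controllers up to date.
; SpawnPlayer destroys the controller's current pawn, spawns a BP_ThirdPersonCharacter at a randomly chosen PlayerStart and possesses it.
; Nothing in this graph calls SpawnPlayer itself.
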(event EventBeginPlay)

(event EventTick
  (params (DeltaSeconds :type Float%20%28single-precision%29)))

(event EventPostLogin
  (params (NewPlayer :type Player%20Controller%20Object%20Reference))
  ;[0 0 0] Player Connection/Disconnection
  ;;[1 1 1] On Player Connects
  (bind _asbp_pc_framework (Utilities|Casting|CastToBP_PC_Framework NewPlayer))
  (Utilities|Array|Add (Variables|Default|GetAll_PCs) _asbp_pc_framework))

(event EventOnSwapPlayerControllers
  (params (OldPC :type Player%20Controller%20Object%20Reference) (NewPC :type Player%20Controller%20Object%20Reference))
  ;[0 0 0] Player Connection/Disconnection
  ;;[1 1 1] On Player Connects
  (Utilities|Array|Add (Variables|Default|GetAll_PCs) NewPC))

(event EventOnLogout
  (params (ExitingController :type Controller%20Object%20Reference))
  ;[0 0 0] Player Connection/Disconnection
  ;;[1 1 1] On Player Disconnect
  (bind _asbp_pc_framework (Utilities|Casting|CastToBP_PC_Framework ExitingController))
  (Utilities|Array|RemoveItem (Variables|Default|GetAll_PCs) _asbp_pc_framework))

(fn ConstructionScript)

(fn FindRandomPlayerStart
  (bind _outactors (Actor|GetAllActorsOfClass "/Script/Engine.PlayerStart"))
  (return (Transformation|GetActorTransform (Utilities|Array|Get(acopy) _outactors (Math|Random|RandomIntegerinRange 0 (- (Utilities|Array|Length _outactors) 1))))))

(fn SpawnPlayer
  (params (Player%20Controller :type Player%20Controller%20Object%20Reference))
  (bind _returnvalue (Pawn|GetControlledPawn Player%20Controller))
  (Utilities|IsValid _returnvalue
    (:Is%20Valid
      (Actor|DestroyActor _returnvalue))
    (:Is%20Not%20Valid
      _))
  (bind _returnvalue_2 (Game|SpawnActorfromClass "/Game/ThirdPerson/Blueprints/BP_ThirdPersonCharacter.BP_ThirdPersonCharacter_C" (Spawning|FindRandomPlayerStart) "Undefined" "MultiplyWithRoot" 0 0))
  (Pawn|Possess Player%20Controller _returnvalue_2))